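; BP_Weapon is a weapon Blueprint that damages actors touched by its DamageCollider.
; On begin overlap, it applies its Damage value to any actor other than its owner, with the owner as damage causer.
; ActivateDamage and DeactivateDamage open and close the hit window by switching the collider between query-only and no collision.
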(event OnComponentBeginOverlap(damagecollider)
  (params (OverlappedComponent :type Primitive%20Component%20Object%20Reference) (OtherActor :type Actor%20Object%20Reference) (OtherComp :type Primitive%20Component%20Object%20Reference) (OtherBodyIndex :type Integer) (bFromSweep :type Boolean) (SweepResult :type Hit%20Result%20Structure%20%28by%20ref%29))
  (if (!= OtherActor (Components|GetOwner))
    (Game|Damage|ApplyDamage OtherActor (Variables|Default|GetDamage) 0 (Components|GetOwner))))

(fn ConstructionScript)

(fn ActivateDamage
  (Collision|SetCollisionEnabled (Variables|Default|Getdamage%20collider) "QueryOnly"))

(fn DeactivateDamage
  (Collision|SetCollisionEnabled (Variables|Default|Getdamage%20collider) "NoCollision"))