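; Player controller that forwards Enhanced Input actions to the possessed BP_PlayerCharacter.
; On possession it caches the character and adds the camera, jump, movement and combat mapping contexts, using each array index as priority.
; Camera input is scaled by sensitivity, while jump, basic combo attack and movement pass to character functions.
; Every handled move phase, including cancel and completion, calls the same movement function.
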(event Input|EnhancedActionEvents|EnhancedInputActionIA_Move
  (params (ActionValue :type Vector%202D%20Structure) (ElapsedSeconds :type Float%20%28double-precision%29) (TriggeredSeconds :type Float%20%28double-precision%29) (InputAction :type Input%20Action%20Object%20Reference :default "/Game/MyContent/Player/Input/IA_Move.IA_Move"))
  ;[1 1 1] Character Movement
  (:Triggered
    (Default|MoveCharacter (Variables|Default|GetChar%20Ref) ActionValue :!label _label))
  (:Started
    (goto _label))
  (:Canceled
    (goto _label))
  (:Completed
    (goto _label)))

(event Input|EnhancedActionEvents|EnhancedInputActionIA_Camera
  (params (ActionValue :type Vector%202D%20Structure) (ElapsedSeconds :type Float%20%28double-precision%29) (TriggeredSeconds :type Float%20%28double-precision%29) (InputAction :type Input%20Action%20Object%20Reference :default "/Game/MyContent/Player/Input/IA_Camera.IA_Camera"))
  ;[1 1 1] Camera Movement
  (Default|ControlCamera (Variables|Default|GetChar%20Ref) (* ActionValue (Variables|Default|GetCameraSensitivity))))

(event Input|EnhancedActionEvents|EnhancedInputActionIA_Jump
  (params (ActionValue :type Boolean) (ElapsedSeconds :type Float%20%28double-precision%29) (TriggeredSeconds :type Float%20%28double-precision%29) (InputAction :type Input%20Action%20Object%20Reference :default "/Game/MyContent/Player/Input/IA_Jump.IA_Jump"))
  ;[1 1 1] Jumping
  (Default|TryJump (Variables|Default|GetChar%20Ref) ActionValue))

(event Input|EnhancedActionEvents|EnhancedInputActionIA_BasicAttack
  (params (ActionValue :type Boolean) (ElapsedSeconds :type Float%20%28double-precision%29) (TriggeredSeconds :type Float%20%28double-precision%29) (InputAction :type Input%20Action%20Object%20Reference :default "/Game/MyContent/Player/Input/IA_BasicAttack.IA_BasicAttack"))
  ;[1 1 1] attack
  (Default|BasicComboAttack (Variables|Default|GetChar%20Ref)))

(event EventPossess
  (params (PossessedPawn :type Pawn%20Object%20Reference))
  ;[1 1 1] Possess character on start (if fails does nothing)
  (bind _asbp_player_character (Utilities|Casting|CastToBP_PlayerCharacter PossessedPawn))
  (Variables|Default|SetChar%20Ref _asbp_player_character)
  (CallFunction|SetDefaultInput))

(fn ConstructionScript)

(fn AddInput
  (params (MappingContext :type Input%20Mapping%20Context%20Object%20Reference) (Priority :type Integer) (Options%20Ignore%20All%20Pressed%20Keys%20Until%20Release :type Boolean))
  (Input|AddMappingContext (PlayerController|LocalPlayerSubsystems|GetEnhancedInputLocalPlayerSubsystem) MappingContext Priority (Utilities|Struct|MakeModifyContextOptions Options%20Ignore%20All%20Pressed%20Keys%20Until%20Release false false)))

(fn SetDefaultInput
  (for (_array_element _array_index) (Utilities|Array|MakeArray "/Game/MyContent/Player/Input/IMC_Camera.IMC_Camera" "/Game/MyContent/Player/Input/IMC_Jump.IMC_Jump" "/Game/MyContent/Player/Input/IMC_Movement.IMC_Movement" "/Game/MyContent/Player/Input/IMC_Combat.IMC_Combat")
    (CallFunction|AddInput _array_element _array_index true)))